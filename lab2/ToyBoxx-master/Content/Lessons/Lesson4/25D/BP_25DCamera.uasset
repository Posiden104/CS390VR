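; BP_25DCamera is a camera Blueprint for a 2.5D lesson that follows player character 0 along the Y and Z axes.
; BeginPlay caches the actor's starting offset from the character and its starting X position.
; Each Tick moves the actor to the character's Y and Z plus that offset, with X held constant at the cached X plus the offset's X.
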(event EventBeginPlay
  (bind _returnvalue (Transformation|GetActorLocation))
  (Variables|Default|SetOffset (- _returnvalue (Transformation|GetActorLocation (Game|GetPlayerCharacter 0))))
  (Variables|Default|SetXLoc (.X (Math|Vector|BreakVector _returnvalue))))

(event EventTick
  (params (DeltaSeconds :type Float%20%28single-precision%29))
  (bind _returnvalue (Game|GetPlayerCharacter 0))
  (bind _returnvalue_2 (Transformation|GetActorLocation _returnvalue))
  (Transformation|SetActorLocation (+ (Math|Vector|MakeVector (Variables|Default|GetXLoc) (.y _returnvalue_2) (.z _returnvalue_2)) (Variables|Default|GetOffset)) false false))

(fn ConstructionScript)