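; BP_TImer is a lesson countdown timer that shows remaining time as a minutes:seconds TextRender and reloads the current level when it runs out.
; A one-second looping timer decrements TimeRemaining, while Tick refreshes the text until HasWon is set.
; A Message event either adds time or sets HasWon and displays the remaining time as the score.
; Winning does not stop the countdown, so the level still reloads at zero.
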(event Custom|DecreaseTimer
  (bind _result (Math|Integer|DecrementInt (Variables|Default|GetTimeRemaining))
    (:%20%20
      (if (<= _result 0)
        (bind _returnvalue (Game|GetCurrentLevelName true))
        (Utilities|FlowControl|Delay 1.0)
        (Game|OpenLevel(byName) (Utilities|String|StringToName _returnvalue))))))

(event EventBeginPlay
  (Utilities|Time|SetTimerbyEvent (delegate Custom|DecreaseTimer) 1.0 (not (Variables|Default|GethasWon))))

(event EventTick
  (params (DeltaSeconds :type Float%20%28single-precision%29))
  (bind _timeremaining (Variables|Default|GetTimeRemaining))
  (bind _returnvalue (/ _timeremaining 60))
  (if (not (Variables|Default|GethasWon))
    (Rendering|Components|TextRender|SetText (Variables|Default|GetTextRender) (Utilities|Text|ToText(String) (Utilities|String|Append "Time Remaining: " (Utilities|String|BuildString(Integer) (Utilities|String|BuildString(Integer) "" "" _returnvalue) ":" (- (Variables|Default|GetTimeRemaining) (* _returnvalue 60))))))))

(event EventMessage
  (params (TimeToAdd :type Integer) (Won :type Boolean))
  (if Won
    (Variables|Default|SethasWon true)
    (Rendering|Components|TextRender|SetText (Variables|Default|GetTextRender) (Utilities|Text|ToText(String) (Utilities|String|Append "Congratulations! Your Score is" (Utilities|String|BuildString(Integer) (Utilities|String|BuildString(Integer) "" "" (/ (Variables|Default|GetTimeRemaining) 60)) ":" (- (Variables|Default|GetTimeRemaining) (* (/ (Variables|Default|GetTimeRemaining) 60) 60))))))
    (else
      (Variables|Default|SetTimeRemaining (+ TimeToAdd (Variables|Default|GetTimeRemaining))))))

(fn ConstructionScript)