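; BP_EnemyTurret is an enemy turret that turns toward and shoots at a SuperHotController pawn it sees.
; PawnSensing sightings snap the actor's rotation to face that pawn.
; If the SpawnProjectile flag is set, it spawns a BP_SuperHotEnemyBullet at ProjSpawnLoc, launches it with a velocity-change impulse and plays a laser sound.
; Random delays on BeginPlay and after each shot re-arm the flag, staggering the fire.
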(event OnSeePawn(PawnSensing)
  (params (Pawn :type Pawn%20Object%20Reference))
  ;[1 1 1] Rotate
  (bind _assuper_hot_controller (Utilities|Casting|CastToSuperHotController Pawn))
  (Utilities|FlowControl|Sequence
    (:then_0
      (Transformation|SetActorRotation (Math|Rotator|FindLookatRotation (Transformation|GetActorLocation) (Transformation|GetActorLocation _assuper_hot_controller))))
    (:then_1
      ;[1 1 1] Shoot
      (if (Variables|Default|GetSpawnProjectile)
        (bind _returnvalue (Game|SpawnActorfromClass "/Game/Blueprints/BP_SuperHotEnemyBullet.BP_SuperHotEnemyBullet_C" (Transformation|GetWorldTransform (Variables|Default|GetProjSpawnLoc)) "Undefined" 0 0))
        (Physics|AddImpulse (Variables|/Game/Blueprints/BP_SuperHotEnemyBullet.BP_SuperHotEnemyBullet_C|GetCube _returnvalue) (* (Math|Vector|GetForwardVector (Variables|Default|GetCube)) 2e+02) "None" true)
        (Audio|SpawnSoundatLocation "/Game/StarterContent/Audio/Laser_Shoot38.Laser_Shoot38" (Transformation|GetWorldLocation (Variables|Default|GetProjSpawnLoc)))
        (Variables|Default|SetSpawnProjectile false)
        (Utilities|FlowControl|Delay (Math|Random|RandomFloatinRange 1.5 3.0))
        (Variables|Default|SetSpawnProjectile true)))))

(event EventBeginPlay
  (Utilities|FlowControl|Delay (Math|Random|RandomFloatinRange 0.5 3.0))
  (Variables|Default|SetSpawnProjectile true))

(fn ConstructionScript)